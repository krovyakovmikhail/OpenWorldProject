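; Minigame controller actor that starts a target minigame when its Interaction function is called.
; Interaction prints a debug message and spawns BP_mini_game_Target_1 actors at six hard-coded positions among twelve placed static meshes.
; A box overlap fills TargetArray with all twelve meshes and clears it on exit, but the spawn logic ignores that array.
; WhoAreYou returns self, while the other query functions are empty stubs.
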(event `self.Box.OnComponentBeginOverlap`
  (params (OverlappedComponent :type "PrimitiveComponent Object Reference") (OtherActor :type "Actor Object Reference") (OtherComp :type "PrimitiveComponent Object Reference") (OtherBodyIndex :type Integer) (bFromSweep :type Boolean) (SweepResult :type "HitResult Structure (by ref)"))
  (set `self.TargetArray` (`|MakeArray` (`self.StaticMesh1`) (`self.StaticMesh2`) (`self.StaticMesh3`) (`self.StaticMesh4`) (`self.StaticMesh5`) (`self.StaticMesh6`) (`self.StaticMesh7`) (`self.StaticMesh8`) (`self.StaticMesh9`) (`self.StaticMesh10`) (`self.StaticMesh11`) (`self.StaticMesh12`))))

(event `self.Box.OnComponentEndOverlap`
  (params (OverlappedComponent :type "PrimitiveComponent Object Reference") (OtherActor :type "Actor Object Reference") (OtherComp :type "PrimitiveComponent Object Reference") (OtherBodyIndex :type Integer))
  (`KismetArrayLibrary.Array_Clear` (`self.TargetArray`)))

(fn `Concretize yourself`
  (returns (Lifted_object :type "/Game/Main/Develop/Interaction_object_base_class/interaction__object_base_class/Lifted_Item_base_class/BP_Lifted_item Object Reference"))
  (return null))

(fn `Interaction`
  (returns (succsses :type Boolean))
  (`KismetSystemLibrary.PrintString` "start game")
  (`|SpawnActorFromClass` "/Game/Main/MiniGame/Minigame_1/BP_mini_game_Target_1.BP_mini_game_Target_1_C" (`KismetMathLibrary.MakeTransform` (`SceneComponent.K2_GetComponentLocation` (`self.StaticMesh1`))) "Undefined" "OverrideRootScale" null null)
  (`|SpawnActorFromClass` "/Game/Main/MiniGame/Minigame_1/BP_mini_game_Target_1.BP_mini_game_Target_1_C" (`KismetMathLibrary.MakeTransform` (`SceneComponent.K2_GetComponentLocation` (`self.StaticMesh2`))) "Undefined" "OverrideRootScale" null null)
  (`|SpawnActorFromClass` "/Game/Main/MiniGame/Minigame_1/BP_mini_game_Target_1.BP_mini_game_Target_1_C" (`KismetMathLibrary.MakeTransform` (`SceneComponent.K2_GetComponentLocation` (`self.StaticMesh5`))) "Undefined" "OverrideRootScale" null null)
  (`|SpawnActorFromClass` "/Game/Main/MiniGame/Minigame_1/BP_mini_game_Target_1.BP_mini_game_Target_1_C" (`KismetMathLibrary.MakeTransform` (`SceneComponent.K2_GetComponentLocation` (`self.StaticMesh7`))) "Undefined" "OverrideRootScale" null null)
  (`|SpawnActorFromClass` "/Game/Main/MiniGame/Minigame_1/BP_mini_game_Target_1.BP_mini_game_Target_1_C" (`KismetMathLibrary.MakeTransform` (`SceneComponent.K2_GetComponentLocation` (`self.StaticMesh10`))) "Undefined" "OverrideRootScale" null null)
  (`|SpawnActorFromClass` "/Game/Main/MiniGame/Minigame_1/BP_mini_game_Target_1.BP_mini_game_Target_1_C" (`KismetMathLibrary.MakeTransform` (`SceneComponent.K2_GetComponentLocation` (`self.StaticMesh11`))) "Undefined" "OverrideRootScale" null null))

(fn `UserConstructionScript`)

(fn `What A Car`
  (returns (Vehicle :type "WheeledVehicle Object Reference"))
  (return null))

(fn `What A Weapon`
  (returns (Weapon :type "/Game/Main/Develop/Interaction_object_base_class/interaction__object_base_class/Lifted_Item_base_class/Class_Weapon/BP_Weapon_Class Object Reference"))
  (return null))

(fn `WhoAreYou`
  (returns (Object :type "/Game/Main/Develop/Interaction_object_base_class/interaction__object_base_class/BP_Interaction_object Object Reference"))
  (return self))