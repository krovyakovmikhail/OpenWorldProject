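; Interactable door actor for MiniGame 2 that swings open when interacted with.
; Interaction calls OpenDoor, which plays a timeline that drives the static mesh's relative yaw, and always returns false.
; CloseDoor_ reverses that timeline, but nothing in this Blueprint calls it.
; WhoAreYou returns the door itself, while the weapon, car and concretize query functions are empty stubs.
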(event `self.Open door`
  (bind (_direction _newtrack_0) (`Timeline|Timeline_2` :!label _label)
    (:`Update`
      (`SceneComponent.K2_SetRelativeRotation` (`self.StaticMesh`) (`KismetMathLibrary.MakeRotator` 0.0 0.0 _newtrack_0) false false))))

(event `Close Door_`
  (goto _label :!via `Reverse`))

(fn `Concretize yourself`
  (returns (Lifted_object :type "/Game/Main/Develop/Interaction_object_base_class/interaction__object_base_class/Lifted_Item_base_class/BP_Lifted_item Object Reference"))
  (return null))

(fn `Interaction`
  (returns (succsses :type Boolean))
  (`self.Open door`)
  (return false))

(fn `UserConstructionScript`
  (`parent.UserConstructionScript`))

(fn `What A Car`
  (returns (Vehicle :type "WheeledVehicle Object Reference"))
  (return null))

(fn `What A Weapon`
  (returns (Weapon :type "/Game/Main/Develop/Interaction_object_base_class/interaction__object_base_class/Lifted_Item_base_class/Class_Weapon/BP_Weapon_Class Object Reference"))
  (return null))

(fn `WhoAreYou`
  (returns (Object :type "/Game/Main/Develop/Interaction_object_base_class/interaction__object_base_class/BP_Interaction_object Object Reference"))
  (return self))