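; Mini-game actor that runs a timed survival challenge against spawned NPCs, started when the open-world character enters the CloseDoor trigger.
; The trigger shuts the door, creates the HUD and countdown, then repeatedly spawns NPCs at the spawn points until the game finishes.
; Reaching the finish trigger wins, while timeout or zero victim health, checked in Updatewidget, loses.
; Either outcome uses delayed timers to remove the widget and destroy the NPCs.
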(event `self.ReceiveTick`
  (params (DeltaSeconds :type "Float (single-precision)")))

(event `Update widget`
  (bind _textblock_health (`/Game/Main/MiniGame/MiniGame_2/WBP_minigame_2.TextBlock_Health` (`self.MiniGame Widget`)))
  (`self.MiniGame Widget`
    (:`then`
      (bind _victim (`self.Victim`)
        (:`then`
          (bind _health (`/Game/Main/Develop/MAIN_CHAR/blueprint/BP_OpenWorld_Character.Health` _victim))
          (if (> _health 0.0)
            (`TextBlock.SetText` _textblock_health (`KismetTextLibrary.Conv_DoubleToText` _health "HalfToEven"))
            (else
              (`TextBlock.SetText` _textblock_health "")
              (`self.Game Over`))))
        (:`else`)))
    (:`else`)))

(event `self.CloseDoor.OnComponentBeginOverlap`
  (params (OverlappedComponent :type "PrimitiveComponent Object Reference") (OtherActor :type "Actor Object Reference") (OtherComp :type "PrimitiveComponent Object Reference") (OtherBodyIndex :type Integer) (bFromSweep :type Boolean) (SweepResult :type "HitResult Structure (by ref)"))
  (bind _asbp_open_world_character (cast `/Game/Main/Develop/MAIN_CHAR/blueprint/BP_OpenWorld_Character` OtherActor))
  (set `self.Victim` _asbp_open_world_character)
  (`/Engine/EditorBlueprintResources/StandardMacros.DoOnce` false
    (:`Completed`
      (`KismetSystemLibrary.PrintString` "Close door")
      (bind _door (`self.Door`)
        (:`then`
          (`/Game/Main/MiniGame/MiniGame_2/BP_interaction_door.Close door` _door)
          (`KismetSystemLibrary.Delay` 2.0)
          (`self.StartGame`)
          (`self.Update widget`)
          (if (not (`self.Finish`)) :!label _label
            (for _array_element (`self.Array_SpawnPoint`)
              (bind _returnvalue (`|SpawnActorFromClass` "/Game/Main/MiniGame/MiniGame_2/TestNPC/BP_NPC.BP_NPC_C" (`KismetMathLibrary.Conv_VectorToTransform` (`self.K2_GetActorLocation` _array_element)) "Undefined" "OverrideRootScale" null null))
              (`KismetArrayLibrary.Array_Add` (`self.Array NPC`) _returnvalue)
              (`KismetSystemLibrary.Delay` 5.0)
              (goto _label))))
        (:`else`)))))

(event `self.Trigger_Finish.OnActorBeginOverlap`
  (params (OverlappedActor :type "Actor Object Reference") (OtherActor :type "Actor Object Reference"))
  (`/Engine/EditorBlueprintResources/StandardMacros.DoOnce` false
    (:`Completed`
      (`self.FinishGame`))))

(fn `Clear Array NPC`
  (`KismetArrayLibrary.Array_Clear` (`self.Array NPC`)))

(fn `ClearNPC`
  (for _array_element (`self.Array NPC`)
    (`/Engine/EditorBlueprintResources/StandardMacros.IsValid` _array_element
      (:`Is Valid`
        (`self.K2_DestroyActor` _array_element)
        (`KismetSystemLibrary.K2_SetTimer` null "Clear Array NPC" 0.5)))))

(fn `FinishGame`
  (bind _minigame_widget (`self.MiniGame Widget`)
    (:`then`
      (`/Game/Main/MiniGame/MiniGame_2/WBP_minigame_2.FinishGame` _minigame_widget)
      (set `self.Finish` true)
      (`KismetSystemLibrary.K2_SetTimer` null "RemoveWidget" 3.0)
      (`KismetSystemLibrary.K2_SetTimer` null "ClearNPC" 3.0))
    (:`else`)))

(fn `Game Over`
  (`/Game/Main/MiniGame/MiniGame_2/WBP_minigame_2.Game Over` (`self.MiniGame Widget`))
  (set `self.Finish` true)
  (`KismetSystemLibrary.K2_SetTimer` null "RemoveWidget" 3.0)
  (`KismetSystemLibrary.K2_SetTimer` null "ClearNPC" 3.5))

(fn `RemoveWidget`
  (`Widget.RemoveFromParent` (`self.MiniGame Widget`))
  (set `self.MiniGame Widget` null))

(fn `StartGame`
  (bind _returnvalue (`|CreateWidget` "/Game/Main/MiniGame/MiniGame_2/WBP_minigame_2.WBP_minigame_2_C"))
  (bind _output_get (set `self.MiniGame Widget` _returnvalue))
  (`UserWidget.AddToViewport` _output_get 0)
  (set `/Game/Main/MiniGame/MiniGame_2/WBP_minigame_2.MiniGame` self _output_get)
  (`KismetSystemLibrary.K2_SetTimer` null "Timer" 1.0 true))

(fn `Timer`
  (if (not (`self.Finish`))
    (if (== (`self.Time`) 0)
      (bind _minigame_widget (`self.MiniGame Widget`)
        (:`then`
          (`/Game/Main/MiniGame/MiniGame_2/WBP_minigame_2.Timer` _minigame_widget 0)
          (`self.Game Over`))
        (:`else`))
      (elif (> (`self.Time`) 0)
        (bind _result (`/Engine/EditorBlueprintResources/StandardMacros.DecrementInt` (`self.Time`))
          (:`  `
            (bind _output_get (set `self.Time` _result))
            (`/Game/Main/MiniGame/MiniGame_2/WBP_minigame_2.Timer` _minigame_widget _output_get)))))))

(fn `UserConstructionScript`)