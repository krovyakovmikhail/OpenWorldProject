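; BP_NPC is a minigame enemy that damages the open-world character when its line of sight reaches them.
; A looping one-second timer fires a short forward debug-drawn trace; hitting the player decrements Health and destroys the NPC.
; It then updates the BP_MiniGame_2 widget and calls a removal on that manager's NPC array.
; A BP_Pellet hit enables mesh physics simulation and switches the capsule to physics-only collision.
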(event `self.ReceiveBeginPlay`
  (bind _outactors (`GameplayStatics.GetAllActorsOfClass` "/Game/Main/MiniGame/MiniGame_2/BP_MiniGame_2.BP_MiniGame_2_C"))
  (set `self.MiniGame` (`|GetArrayItem` _outactors))
  (bind _outactors_2 (`GameplayStatics.GetAllActorsOfClass` "/Game/Main/Develop/MAIN_CHAR/blueprint/BP_OpenWorld_Character.BP_OpenWorld_Character_C"))
  (set `self.Target` (`|GetArrayItem` _outactors_2))
  (`KismetSystemLibrary.K2_SetTimerDelegate` (delegate `TRace`) 1.0 true))

(event `TRace`
  (bind _returnvalue (`self.K2_GetActorLocation`))
  (bind _outhit (`KismetSystemLibrary.LineTraceSingle` :`Start` _returnvalue :`End` (+ _returnvalue (* (`self.GetActorForwardVector`) 200.0)) :`TraceChannel` "TraceTypeQuery1" :`DrawDebugType` "ForDuration" :`DrawTime` 3.0))
  (bind _target (`self.Target`)
    (:`then`
      (if (== (`.HitActor` (`GameplayStatics.BreakHitResult` _outhit)) (`self.Target`))
        (bind _result (`/Engine/EditorBlueprintResources/StandardMacros.DecrementFloat` (`/Game/Main/Develop/MAIN_CHAR/blueprint/BP_OpenWorld_Character.Health` _target))
          (:`  `
            (set `/Game/Main/Develop/MAIN_CHAR/blueprint/BP_OpenWorld_Character.Health` _result _target)
            (`self.K2_DestroyActor`)
            (bind _minigame (`self.MiniGame`)
              (:`then`
                (`/Game/Main/MiniGame/MiniGame_2/BP_MiniGame_2.Update widget` _minigame)
                (`KismetArrayLibrary.Array_RemoveItem` (`/Game/Main/MiniGame/MiniGame_2/BP_MiniGame_2.Array NPC` _minigame)))
              (:`else`))))))
    (:`else`)))

(event `self.CapsuleComponent.OnComponentHit`
  (params (HitComponent :type "PrimitiveComponent Object Reference") (OtherActor :type "Actor Object Reference") (OtherComp :type "PrimitiveComponent Object Reference") (NormalImpulse :type "Vector Structure") (Hit :type "HitResult Structure (by ref)"))
  (if (== (`GameplayStatics.GetObjectClass` OtherActor) "/Game/Main/Develop/Weapon/Shotgun/blueprint/BP_Pellet.BP_Pellet_C")
    (`PrimitiveComponent.SetSimulatePhysics` (`self.Mesh`) true)
    (`PrimitiveComponent.SetCollisionEnabled` (`self.CapsuleComponent`) "PhysicsOnly")))

(fn `UserConstructionScript`)