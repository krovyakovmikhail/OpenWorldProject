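; BP_interaction_door is an interactable minigame door that toggles open and closed by rotating its static mesh in yaw.
; Interaction calls OpenDoor or CloseDoor based on IsOpen, each driven by its own timeline, while WhoAreYou returns the actor itself.
; IsActive blocks interaction during opening only, since the closing timeline sets it false on every update.
; IsOpen flips as soon as either timeline starts updating.
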(event `Open door`
  (bind (_direction _newtrack_0) (`Timeline|Timeline_0`)
    (:`Update`
      (set `self.isActive` true)
      (`SceneComponent.K2_SetRelativeRotation` (`self.StaticMesh`) (`KismetMathLibrary.MakeRotator` 0.0 0.0 _newtrack_0) false false)
      (set `self.isOpen` true))
    (:`Finished`
      (set `self.isActive` false :!label _label))))

(event `Close door`
  (bind (_direction _newtrack_0) (`Timeline|Timeline_1`)
    (:`Update`
      (set `self.isActive` false)
      (`SceneComponent.K2_SetRelativeRotation` (`self.StaticMesh`) (`KismetMathLibrary.MakeRotator` 0.0 0.0 _newtrack_0) false false)
      (set `self.isOpen` false))
    (:`Finished`
      (goto _label))))

(fn `Interaction`
  (returns (succsses :type Boolean))
  (if (not (`self.isActive`))
    (if (`self.isOpen`)
      (`self.Close door`)
      (else
        (`self.Open door`)))
    (return false)))

(fn `UserConstructionScript`)

(fn `WhoAreYou`
  (returns (Object :type "/Game/Main/Develop/Interaction_object_base_class/interaction__object_base_class/BP_Interaction_object Object Reference"))
  (return self))