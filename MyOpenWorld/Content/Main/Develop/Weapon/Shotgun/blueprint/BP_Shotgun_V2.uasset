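; Shotgun weapon actor that fires a spread of physics pellets and can show an aim point.
; Fire sets the Shoot flag, spawns six BP_Pellets pushed along separate muzzle points' forward vectors, plays shot effects and starts a short timer.
; The pellet spawns are unrolled calls because, per an in-graph note, looping spawned only the first.
; The Reload event plays a sound, then clears Shoot after a delay.
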(event `self.ReceiveActorBeginOverlap`
  (params (OtherActor :type "Actor Object Reference"))
  (`parent.ReceiveActorBeginOverlap` OtherActor)
  (set `self.BulletPoints` (`|MakeArray` (`self.BulletPoint`) (`self.BulletPoint1`) (`self.BulletPoint3`))))

(event `Event Reload`
  (`GameplayStatics.PlaySoundAtLocation` "/Game/Main/Develop/Weapon/Shotgun/Sound/chelovek-zaryadil-drobovik-obrez-6848.chelovek-zaryadil-drobovik-obrez-6848" (`self.K2_GetActorLocation`) (struct) 1.0 1.0 0.0 null null null)
  (`KismetSystemLibrary.Delay` 1.0)
  (set `self.Shoot` false))

(event `/Game/Main/Develop/Interaction_object_base_class/interaction__object_base_class/Lifted_Item_base_class/BP_Lifted_item.AIM`
  (params (`char ` :type "/Game/Main/Develop/MAIN_CHAR/blueprint/BP_OpenWorld_Character Object Reference"))
  (`SceneComponent.SetVisibility` (`self.AimPoint`) true false))

(event `self.Sphere.OnComponentBeginOverlap`
  (params (OverlappedComponent :type "PrimitiveComponent Object Reference") (OtherActor :type "Actor Object Reference") (OtherComp :type "PrimitiveComponent Object Reference") (OtherBodyIndex :type Integer) (bFromSweep :type Boolean) (SweepResult :type "HitResult Structure (by ref)")))

(event `self.Sphere.OnComponentEndOverlap`
  (params (OverlappedComponent :type "PrimitiveComponent Object Reference") (OtherActor :type "Actor Object Reference") (OtherComp :type "PrimitiveComponent Object Reference") (OtherBodyIndex :type Integer)))

(fn `Aiming `
  (params (Char :type "/Game/Main/Develop/MAIN_CHAR/blueprint/BP_OpenWorld_Character Object Reference"))
  (`SceneComponent.SetVisibility` (`self.AimPoint`) true false))

(fn `Concretize yourself`
  (returns (Lifted_object :type "/Game/Main/Develop/Interaction_object_base_class/interaction__object_base_class/Lifted_Item_base_class/BP_Lifted_item Object Reference"))
  (return self))

(fn `Fire`
  (locals (`the speed of the shot` :type "Float (double-precision)" :default 90000.0))
  (bind _returnvalue (`SceneComponent.K2_GetComponentLocation` (`self.BulletPoint`)))
  (set `self.Shoot` true)
  ;[1 1 1] Не получается через цикл вывести, спаунится только первый
  (`self.spawn_bullet` (`local.the speed of the shot`) (`self.BulletPoint`))
  (`self.spawn_bullet` (`local.the speed of the shot`) (`self.BulletPoint1`))
  (`self.spawn_bullet` (`local.the speed of the shot`) (`self.BulletPoint2`))
  (`self.spawn_bullet` (`local.the speed of the shot`) (`self.BulletPoint3`))
  (`self.spawn_bullet` (`local.the speed of the shot`) (`self.BulletPoint4`))
  (`self.spawn_bullet` (`local.the speed of the shot`) (`self.BulletPoint6`))
  (`KismetSystemLibrary.K2_SetTimerDelegate` (`|CreateDelegate` :!event `Event Reload`) 0.5)
  (`GameplayStatics.PlaySoundAtLocation` "/Game/Main/Develop/Weapon/Shotgun/Sound/odinochnyiy-vyistrel-iz-drobovika-na-otkryitoy-ploschadke-6857.odinochnyiy-vyistrel-iz-drobovika-na-otkryitoy-ploschadke-6857" _returnvalue (struct) 1.0 1.0 0.0 null null null)
  (`GameplayStatics.SpawnEmitterAtLocation` "/Game/StarterContent/Particles/P_Explosion.P_Explosion" _returnvalue (struct :`Yaw` 90.0) (0.15 0.15 0.15)))

(fn `Interaction`
  (returns (succsses :type Boolean))
  (return false))

(fn `Reload`)

(fn `spawn_bullet`
  (params (B :type "Float (double-precision)") (BulletPoint :type "ArrowComponent Object Reference"))
  (bind _returnvalue (`|SpawnActorFromClass` "/Game/Main/Develop/Weapon/Shotgun/blueprint/BP_Pellet.BP_Pellet_C" (`KismetMathLibrary.MakeTransform` (`SceneComponent.GetSocketLocation` BulletPoint "None") (struct) (0.2 0.2 0.2)) "AlwaysSpawn" "OverrideRootScale" null null))
  (`PrimitiveComponent.AddForce` (`/Game/Main/Develop/Weapon/Shotgun/blueprint/BP_Pellet.StaticMesh` _returnvalue) (* (`SceneComponent.GetForwardVector` BulletPoint) B) "None" false))

(fn `UserConstructionScript`
  (`parent.UserConstructionScript`))

(fn `What A Car`
  (returns (Vehicle :type "WheeledVehicle Object Reference"))
  (return null))

(fn `What A Weapon`
  (returns (Weapon :type "/Game/Main/Develop/Interaction_object_base_class/interaction__object_base_class/Lifted_Item_base_class/Class_Weapon/BP_Weapon_Class Object Reference"))
  (return self))

(fn `WhoAreYou`
  (returns (Object :type "/Game/Main/Develop/Interaction_object_base_class/interaction__object_base_class/BP_Interaction_object Object Reference"))
  (return self))