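; MK2 grenade actor, an interaction object that explodes on a fuse once triggered.
; The Explosion event sets a three-second timer by function name targeting Explosion.
; The Explosion function spawns a particle effect and sound at the actor's location, fires a RadialForce impulse, then destroys the actor.
; Interaction returns false, while WhoAreYou and ConcretizeYourself return the grenade itself.
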(event `Event Explosion`
  (`KismetSystemLibrary.K2_SetTimer` null "Explosion" 3.0))

(fn `Concretize yourself`
  (returns (Lifted_object :type "/Game/Main/Develop/Interaction_object_base_class/interaction__object_base_class/Lifted_Item_base_class/BP_Lifted_item Object Reference"))
  (return self))

(fn `Explosion`
  (bind _returnvalue (`self.K2_GetActorLocation`))
  (`GameplayStatics.SpawnEmitterAtLocation` "/Game/StarterContent/Particles/P_Explosion.P_Explosion" _returnvalue)
  (`GameplayStatics.PlaySoundAtLocation` "/Game/StarterContent/Audio/Explosion01.Explosion01" _returnvalue (struct) 1.0 1.0 0.0 null null null)
  (`RadialForceComponent.FireImpulse` (`self.RadialForce`))
  (`self.K2_DestroyActor`))

(fn `Interaction`
  (returns (succsses :type Boolean))
  (return false))

(fn `UserConstructionScript`
  (`parent.UserConstructionScript`))

(fn `WhoAreYou`
  (returns (Object :type "/Game/Main/Develop/Interaction_object_base_class/interaction__object_base_class/BP_Interaction_object Object Reference"))
  (return self))