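; Drivable boat pawn that the player boards through an interaction, bringing along an AI companion if one exists.
; SitDown disables capsule collision, attaches character and friend to seat components, flags the Enrique AI controller as InCar and possesses the boat.
; Forward input applies mesh impulses, while steering directly adds yaw rotation to the mesh.
; Pressing Interaction calls StandUp, which detaches both, restores collision, repossesses the character and restarts companion movement.
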(event `self.ReceiveTick`
  (params (DeltaSeconds :type "Float (single-precision)")))

(event `InputAxis|MoveForward`
  (params (AxisValue :type "Float (single-precision)"))
  (`PrimitiveComponent.AddImpulse` (`self.StaticMesh`) (* (* (`self.GetActorForwardVector`) AxisValue) (`self.MoveSpeed `)) "None" false))

(event `InputAxis|MoveRight`
  (params (AxisValue :type "Float (single-precision)"))
  (`SceneComponent.K2_AddRelativeRotation` (`self.StaticMesh`) (`KismetMathLibrary.MakeRotator` 0.0 0.0 (/ AxisValue 5.0)) false false))

(event `InputAction|Interaction`
  (params (Key :type "Key Structure"))
  (:`Pressed`
    (bind _char (`self.Char`)
      (:`then`
        (`self.Stand Up` _char))
      (:`else`))))

(event `/Game/Main/Develop/Boat/Boat1/BPI_boat_interface.Interaction`
  (params (Char :type "/Game/Main/Develop/MAIN_CHAR/blueprint/BP_OpenWorld_Character Object Reference"))
  (bind _output_get (set `self.Char` Char))
  (if (not (`self.OnBoard`))
    (`self.sit down` _output_get)))

(fn `sit down`
  (params (char :type "/Game/Main/Develop/MAIN_CHAR/blueprint/BP_OpenWorld_Character Object Reference"))
  (bind _friend (`/Game/Main/Develop/MAIN_CHAR/blueprint/BP_OpenWorld_Character.Friend` char)
    (:`then`
      (`PrimitiveComponent.SetCollisionEnabled` (`Character.CapsuleComponent` _friend) "NoCollision")
      (`self.K2_AttachToComponent` _friend (`self.seetPassendger`) "None" "SnapToTarget" "SnapToTarget" "SnapToTarget" false)
      (bind _asbp_ai_controller_enrique (cast `/Game/Main/Develop/AI_Enrique/Blueprint/BP_AI_Controller_Enrique` (`AIBlueprintHelperLibrary.GetAIController` _friend)))
      (set `/Game/Main/Develop/AI_Enrique/Blueprint/BP_AI_Controller_Enrique.inCar` true _asbp_ai_controller_enrique))
    (:`else`
      _))
  (`PrimitiveComponent.SetCollisionEnabled` (`Character.CapsuleComponent` char) "NoCollision")
  (`self.K2_AttachToComponent` char (`self.SeetDriver`) "None" "SnapToTarget" "SnapToTarget" "SnapToTarget" false)
  (set `/Game/Main/Develop/MAIN_CHAR/blueprint/BP_OpenWorld_Character.OnDrive` true char)
  (`Controller.Possess` (`GameplayStatics.GetPlayerController` 0) self)
  (set `self.OnBoard` true))

(fn `Stand Up`
  (params (Char :type "/Game/Main/Develop/MAIN_CHAR/blueprint/BP_OpenWorld_Character Object Reference"))
  (bind _returnvalue (`GameplayStatics.GetPlayerController` 0))
  (set `self.OnBoard` false)
  (`Controller.UnPossess` _returnvalue)
  (`self.K2_DetachFromActor` Char "KeepWorld" "KeepWorld" "KeepWorld")
  (set `/Game/Main/Develop/MAIN_CHAR/blueprint/BP_OpenWorld_Character.OnDrive` false Char)
  (`Controller.Possess` _returnvalue Char)
  (`PrimitiveComponent.SetCollisionEnabled` (`Character.CapsuleComponent` Char) "QueryAndPhysics")
  (bind _friend (`/Game/Main/Develop/MAIN_CHAR/blueprint/BP_OpenWorld_Character.Friend` Char)
    (:`then`
      (`self.K2_DetachFromActor` _friend "KeepWorld" "KeepWorld" "KeepWorld")
      (`PrimitiveComponent.SetCollisionEnabled` (`Character.CapsuleComponent` _friend) "QueryAndPhysics")
      (bind _asbp_ai_controller_enrique (cast `/Game/Main/Develop/AI_Enrique/Blueprint/BP_AI_Controller_Enrique` (`AIBlueprintHelperLibrary.GetAIController` _friend)))
      (set `/Game/Main/Develop/AI_Enrique/Blueprint/BP_AI_Controller_Enrique.inCar` false _asbp_ai_controller_enrique)
      (`/Game/Main/Develop/AI_Enrique/Blueprint/BP_AI_Controller_Enrique.RestartMove` _asbp_ai_controller_enrique))
    (:`else`)))

(fn `UserConstructionScript`)