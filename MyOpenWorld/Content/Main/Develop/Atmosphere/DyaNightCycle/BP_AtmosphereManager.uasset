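; Atmosphere manager that drives a day-night cycle by rotating the directional light and changing the sky light color.
; Tick scales CycleSpeed by delta time into a step, which a looping 0.05-second timer adds to the sun's pitch and yaw.
; The timer also sets the star sky's rotation from that step and prints sun angles.
; Two pitch and yaw windows near the horizon each play a timeline that sets sky light brightness.
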(event `self.ReceiveBeginPlay`
  (`KismetSystemLibrary.K2_SetTimerDelegate` (delegate `SunRotation`) 0.05 true))

(event `SunRotation`
  (bind _currentlocation (`self.CurrentLocation`))
  (bind _currentlocation_2 (`self.CurrentLocation`))
  (bind (_returnvalue_roll _returnvalue_pitch _returnvalue_yaw) (`KismetMathLibrary.BreakRotator` (`SceneComponent.K2_GetComponentRotation` (`Light.LightComponent` (`self.DirectionalLight`)))))
  (bind _directionallight (`self.DirectionalLight`)
    (:`then`
      (`self.K2_AddActorWorldRotation` _directionallight (`KismetMathLibrary.MakeRotator` 0.0 _currentlocation _currentlocation) false false)
      (bind _sky_stars (`self.Sky_stars`)
        (:`then`
          (`self.K2_SetActorRelativeRotation` _sky_stars (`KismetMathLibrary.MakeRotator` 0.0 (/ _currentlocation_2 2.0) _currentlocation_2) false false)
          (`KismetSystemLibrary.PrintString` (`KismetStringLibrary.Conv_DoubleToString` _returnvalue_pitch) true true (struct :`G` 1.0 :`B` 0.25 :`A` 1.0) 30.0)
          (`KismetSystemLibrary.PrintString` (`KismetStringLibrary.Conv_DoubleToString` _returnvalue_yaw) true true (struct :`G` 0.410087 :`B` 1.0 :`A` 1.0) 30.0)
          (if (and (< _returnvalue_pitch -0.0) (> _returnvalue_pitch -15.0) (> _returnvalue_yaw 118.0))
            (bind _skylight (`self.SkyLight`)
              (:`then`
                (bind (_direction _newtrack_0) (`Timeline|Timeline_1`)
                  (:`Update`
                    (bind _lightcomponent (`SkyLight.LightComponent` _skylight))
                    (`SkyLightComponent.SetLightColor` _lightcomponent (make `LinearColor` _newtrack_0 _newtrack_0 _newtrack_0 _newtrack_0)))))
              (:`else`))
            (elif (and (> _returnvalue_pitch -15.0) (< _returnvalue_pitch 0.0) (< _returnvalue_yaw 40.0))
              (`self.SkyLight`
                (:`then`
                  (bind (_direction_2 _newtrack_0_2) (`Timeline|Timeline_0`)
                    (:`Update`
                      (`SkyLightComponent.SetLightColor` _lightcomponent (make `LinearColor` _newtrack_0_2 _newtrack_0_2 _newtrack_0_2 _newtrack_0_2)))))
                (:`else`)))))
        (:`else`)))
    (:`else`)))

(event `self.ReceiveTick`
  (params (DeltaSeconds :type "Float (single-precision)"))
  (set `self.CurrentLocation` (* DeltaSeconds (`self. CycleSpeed`))))

(fn `UserConstructionScript`)