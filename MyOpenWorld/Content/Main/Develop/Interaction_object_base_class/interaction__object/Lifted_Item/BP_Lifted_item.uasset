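; BP_Lifted_item is an interaction object for liftable items, with most of its functions left as stubs.
; Aiming previews a throw arc from the character's ThrowLevel using projectile path prediction against WorldStatic, shown through debug drawing.
; It then moves a component to a fixed location and makes it visible, without using the prediction result.
; The throw event, Trow and Interaction hold no logic, and ConcretizeYourself returns self.
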(event `throw`)

(fn `Aiming`
  (params (Char :type "/Game/Main/Develop/MAIN_CHAR/blueprint/BP_OpenWorld_Character Object Reference"))
  (returns (succsses :type Boolean))
  (bind (_returnvalue_location _returnvalue_rotation) (`KismetMathLibrary.BreakTransform` (`SceneComponent.K2_GetComponentToWorld` (`/Game/Main/Develop/MAIN_CHAR/blueprint/BP_OpenWorld_Character.throw level` Char))))
  (`GameplayStatics.Blueprint_PredictProjectilePath_ByObjectType` :`StartPos` _returnvalue_location :`LaunchVelocity` (* (`KismetMathLibrary.GetForwardVector` _returnvalue_rotation) 1500.0) :`ProjectileRadius` 5.0 :`ObjectTypes` (`|MakeArray` "ObjectTypeQuery1" :!type "EObjectTypeQuery Enum") :`DrawDebugType` "ForDuration" :`SimFrequency` 10.0)
  (`SceneComponent.K2_SetWorldLocation` (1000.0 0.0 0.0))
  (`SceneComponent.SetVisibility` true)
  (return false))

(fn `Concretize yourself`
  (returns (Lifted_object :type "/Game/Main/Develop/Interaction_object_base_class/interaction__object/Lifted_Item/BP_Lifted_item Object Reference"))
  (return self))

(fn `Interaction`
  (returns (succsses :type Boolean))
  (return false))

(fn `trow`
  (returns (Succsses :type Boolean))
  (return false))

(fn `UserConstructionScript`
  (`parent.UserConstructionScript`))

(fn `WhatACar`
  (returns (Vehicle :type "WheeledVehicle Object Reference"))
  (return null))

(fn `WhoAreYou`
  (returns (Object :type "/Game/Main/Develop/Interaction_object_base_class/interaction__object/BP_Interaction_object Object Reference"))
  (return null))