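; Base Blueprint for a lifted item that a character can aim and throw, with a landing marker shown while aiming.
; AIM opens a Tick gate so Aiming predicts a projectile path from the character's ThrowLevel each frame and moves their decal to its end, with debug drawing enabled.
; Throw only hides the decal and closes the gate.
; Explosion and most query functions are empty stubs, while ConcretizeYourself returns self.
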(event `self.ReceiveTick`
  (params (DeltaSeconds :type "Float (single-precision)"))
  (`parent.ReceiveTick` DeltaSeconds)
  (`/Engine/EditorBlueprintResources/StandardMacros.Gate` true :!label _label
    (:`Exit`
      (`self.Aiming ` (stale `AIM` `char `)))))

(event `AIM`
  (params (`char ` :type "/Game/Main/Develop/MAIN_CHAR/blueprint/BP_OpenWorld_Character Object Reference"))
  (goto _label :!via `Open`))

(event `Throw`
  (if (`KismetSystemLibrary.IsValid` (stale `AIM` `char `))
    (`SceneComponent.SetVisibility` (`/Game/Main/Develop/MAIN_CHAR/blueprint/BP_OpenWorld_Character.Decal` (stale `AIM` `char `)) false false)
    (goto _label :!via `Close`)))

(event `Event Explosion`)

(fn `Aiming `
  (params (Char :type "/Game/Main/Develop/MAIN_CHAR/blueprint/BP_OpenWorld_Character Object Reference"))
  (bind _decal (`/Game/Main/Develop/MAIN_CHAR/blueprint/BP_OpenWorld_Character.Decal` Char))
  (bind (_returnvalue_location _returnvalue_rotation) (`KismetMathLibrary.BreakTransform` (`SceneComponent.K2_GetComponentToWorld` (`/Game/Main/Develop/MAIN_CHAR/blueprint/BP_OpenWorld_Character.throw level` Char))))
  (if (`KismetSystemLibrary.IsValid` Char)
    (bind (_outhit _outpathpositions _outlasttracedestination) (`GameplayStatics.Blueprint_PredictProjectilePath_ByObjectType` :`StartPos` _returnvalue_location :`LaunchVelocity` (* (`KismetMathLibrary.GetForwardVector` _returnvalue_rotation) 1500.0) :`ProjectileRadius` 5.0 :`ObjectTypes` (`|MakeArray` "ObjectTypeQuery1" :!type "EObjectTypeQuery Enum") :`DrawDebugType` "ForDuration" :`SimFrequency` 10.0))
    (`SceneComponent.K2_SetWorldLocation` _decal _outlasttracedestination false false)
    (`SceneComponent.SetVisibility` _decal true false)))

(fn `Concretize yourself`
  (returns (Lifted_object :type "/Game/Main/Develop/Interaction_object_base_class/interaction__object_base_class/Lifted_Item_base_class/BP_Lifted_item Object Reference"))
  (return self))

(fn `Interaction`
  (returns (succsses :type Boolean))
  (return false))

(fn `UserConstructionScript`
  (`parent.UserConstructionScript`))

(fn `What A Car`
  (returns (Vehicle :type "WheeledVehicle Object Reference"))
  (return null))

(fn `What A Weapon`
  (returns (Weapon :type "/Game/Main/Develop/Interaction_object_base_class/interaction__object_base_class/Lifted_Item_base_class/Class_Weapon/BP_Weapon_Class Object Reference"))
  (return null))

(fn `WhoAreYou`
  (returns (Object :type "/Game/Main/Develop/Interaction_object_base_class/interaction__object_base_class/BP_Interaction_object Object Reference"))
  (return null))