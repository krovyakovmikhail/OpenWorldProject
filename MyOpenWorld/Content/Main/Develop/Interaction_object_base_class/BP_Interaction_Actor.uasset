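; BP_Interaction_Actor is a base actor class for interactable objects, kept in the interaction object base class folder.
; It declares stub functions for interacting, firing, getting in a car with a driver and controller, identity queries and a test.
; Every body is empty or returns false, and the events and construction script do nothing, so it holds no behavior of its own.
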(fn `Fire`
  (returns (shoot :type Boolean))
  (return false))

(fn `get in the car`
  (params (Driver :type "/Game/Main/Develop/MAIN_CHAR/blueprint/BP_OpenWorld_Character Object Reference") (MainController :type "PlayerController Object Reference"))
  (returns (Succsess :type Boolean))
  (return false))

(fn `Interact`
  (returns (Succsess :type Boolean))
  (return false))

(fn `TestFunction`
  (returns (Succsses :type Boolean))
  (return false))

(fn `UserConstructionScript`)

(fn `what a car`
  (returns (`transport vehicle` :type "WheeledVehicle Object Reference"))
  (return null))

(fn `WhoAreYou`
  (returns (ReferenceOnInteractActor :type "/Game/Main/Develop/Interaction_object_base_class/BP_Interaction_Actor Object Reference"))
  (return null))