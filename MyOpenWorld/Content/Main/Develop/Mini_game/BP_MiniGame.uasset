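; BP_MiniGame is an interactable target minigame that respawns its targets and liftable projectile objects on each start.
; Interact destroys existing objects, spawns BP_Target and Interactable_lifted_object at marker actor locations, and briefly shows an intro widget.
; Target cleanup is nested inside the projectile loop, so it needs at least one existing projectile.
; UpdateGame removes targets from the tracked list and shows a temporary win widget when it empties.
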(event `self.ReceiveBeginPlay`)

(event `WIN`
  (bind _returnvalue (`|CreateWidget` "/Game/Main/Develop/Mini_game/WBP_MiniGame_WIN.WBP_MiniGame_WIN_C"))
  (`UserWidget.AddToViewport` _returnvalue 0)
  (`KismetSystemLibrary.Delay` 2.0)
  (`Widget.RemoveFromParent` _returnvalue))

(event `InteractableObject_Interface.Interact`
  (params (ActorInteractedWithObject :type "Actor Object Reference"))
  (`self.Start Game`)
  (bind _returnvalue (`|CreateWidget` "/Game/Main/Develop/Mini_game/WBP_MiniGame.WBP_MiniGame_C"))
  (`UserWidget.AddToViewport` _returnvalue 0)
  (`KismetSystemLibrary.Delay` 4.0)
  (`Widget.RemoveFromParent` _returnvalue))

(fn `PreparingForNewGame`
  (bind _outactors (`GameplayStatics.GetAllActorsOfClass` "/Game/Main/Develop/Interactable_Object/Interactable_lifted_object.Interactable_lifted_object_C"))
  (for _array_element _outactors
    (`self.K2_DestroyActor` _array_element)
    (bind _outactors_2 (`GameplayStatics.GetAllActorsOfClass` "/Game/Main/Develop/Mini_game/BP_target.BP_Target_C"))
    (for _array_element_2 _outactors_2
      (`self.K2_DestroyActor` _array_element_2)
      (`KismetArrayLibrary.Array_Clear` (`self.Targets`)))))

(fn `Start Game`
  (`self.PreparingForNewGame`)
  (`|ExecutionSequence`
    (:`then_0`
      (for _array_element (`self.ArrayTargets`)
        (bind _returnvalue_location (`KismetMathLibrary.BreakTransform` (`SceneComponent.K2_GetComponentToWorld` (`Actor.RootComponent` _array_element))))
        (bind _returnvalue (`|SpawnActorFromClass` "/Game/Main/Develop/Mini_game/BP_target.BP_Target_C" (`KismetMathLibrary.MakeTransform` _returnvalue_location (struct) (0.0825 0.245 0.455)) "Undefined" "OverrideRootScale" null null))
        (set `/Game/Main/Develop/Mini_game/BP_target.Mini_Game` self _returnvalue)
        (`KismetArrayLibrary.Array_AddUnique` (`self.Targets`) _returnvalue)))
    (:`then_1`
      (for _array_element_2 (`self.ArrayProjectile`)
        (bind _returnvalue_location_2 (`KismetMathLibrary.BreakTransform` (`SceneComponent.K2_GetComponentToWorld` (`Actor.RootComponent` _array_element_2))))
        (`|SpawnActorFromClass` "/Game/Main/Develop/Interactable_Object/Interactable_lifted_object.Interactable_lifted_object_C" (`KismetMathLibrary.MakeTransform` _returnvalue_location_2) "Undefined" "OverrideRootScale" null null)))))

(fn `UpdateGame`
  (params (BP_Target :type Boolean) (Target_Box :type "Object Object Reference"))
  (returns (Succsess :type Boolean))
  (bind _targets (`self.Targets`))
  (`KismetArrayLibrary.Array_RemoveItem` _targets Target_Box)
  (if (== (`KismetArrayLibrary.Array_Length` _targets) 0)
    (`self.WIN`)
    (return false)))

(fn `UserConstructionScript`)