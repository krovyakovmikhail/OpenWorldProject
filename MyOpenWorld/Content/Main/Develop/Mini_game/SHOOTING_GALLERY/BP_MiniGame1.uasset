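; Shooting gallery mini-game Blueprint that spawns targets on interaction and shows a win screen.
; Interact runs StartGame, which clears old targets and pots, then spawns both target types and pots at marker locations from three arrays.
; Cleanup loops are nested, so child targets and pots are only destroyed while BP_Target_figure actors exist.
; UpdateGame removes entries from a separate Targets array and calls WIN when empty, briefly displaying the win widget.
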(event `self.ReceiveBeginPlay`)

(event `WIN`
  (bind _returnvalue (`|CreateWidget` "/Game/Main/Develop/Mini_game/WBP_MiniGame_WIN.WBP_MiniGame_WIN_C"))
  (`UserWidget.AddToViewport` _returnvalue 0)
  (`KismetSystemLibrary.Delay` 2.0)
  (`Widget.RemoveFromParent` _returnvalue))

(event `InteractableObject_Interface.Interact`
  (params (ActorInteractedWithObject :type "Actor Object Reference"))
  (`self.Start Game`))

(fn `PreparingForNewGame`
  (bind _outactors (`GameplayStatics.GetAllActorsOfClass` "/Game/Main/Develop/Mini_game/SHOOTING_GALLERY/BP_Target_figure.BP_Target_figure_C"))
  (for _array_element _outactors
    (`self.K2_DestroyActor` _array_element)
    (bind _outactors_2 (`GameplayStatics.GetAllActorsOfClass` "/Game/Main/Develop/Mini_game/SHOOTING_GALLERY/BP_Target_figure_Child.BP_Target_figure_Child_C"))
    (for _array_element_2 _outactors_2
      (`self.K2_DestroyActor` _array_element_2)
      (bind _outactors_3 (`GameplayStatics.GetAllActorsOfClass` "/Game/Main/Develop/Mini_game/SHOOTING_GALLERY/BP_Pot.BP_Pot_C"))
      (for _array_element_3 _outactors_3
        (`self.K2_DestroyActor` _array_element_3)))))

(fn `Start Game`
  (`self.PreparingForNewGame`)
  (`|ExecutionSequence`
    (:`then_0`
      (for _array_element (`self.ArrayTargets2`)
        (`|SpawnActorFromClass` "/Game/Main/Develop/Mini_game/SHOOTING_GALLERY/BP_Target_figure_Child.BP_Target_figure_Child_C" (`KismetMathLibrary.MakeTransform` (`SceneComponent.K2_GetComponentLocation` (`Actor.RootComponent` _array_element)) (struct) (0.3 0.3 0.2)) "Undefined" "OverrideRootScale" null null)))
    (:`then_1`
      (for _array_element_2 (`self.ArrayTargets1`)
        (`|SpawnActorFromClass` "/Game/Main/Develop/Mini_game/SHOOTING_GALLERY/BP_Target_figure.BP_Target_figure_C" (`KismetMathLibrary.MakeTransform` (`SceneComponent.K2_GetComponentLocation` (`Actor.RootComponent` _array_element_2))) "Undefined" "OverrideRootScale" null null)))
    (:`then_2`
      (for _array_element_3 (`self.ArrayTargets3`)
        (`|SpawnActorFromClass` "/Game/Main/Develop/Mini_game/SHOOTING_GALLERY/BP_Pot.BP_Pot_C" (`KismetMathLibrary.MakeTransform` (`SceneComponent.K2_GetComponentLocation` (`Actor.RootComponent` _array_element_3)) (struct) (0.1025 0.1025 0.21)) "Undefined" "OverrideRootScale" null null)))))

(fn `UpdateGame`
  (params (BP_Target :type Boolean) (Target_Box :type "Object Object Reference"))
  (returns (Succsess :type Boolean))
  (bind _targets (`self.Targets`))
  (`KismetArrayLibrary.Array_RemoveItem` _targets Target_Box)
  (if (== (`KismetArrayLibrary.Array_Length` _targets) 0)
    (`self.WIN`)
    (return false)))

(fn `UserConstructionScript`)