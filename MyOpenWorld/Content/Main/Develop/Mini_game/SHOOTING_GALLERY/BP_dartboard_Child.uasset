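; Child dartboard Blueprint for the shooting gallery mini-game, extending its parent dartboard.
; On BeginPlay it runs the parent logic, then computes the Cube's world roll offset by half a turn.
; The Cube's hit event is empty, and a delayed rotation reset using that roll is disconnected, so it never runs.
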(event `self.ReceiveBeginPlay`
  (bind _returnvalue_roll (`KismetMathLibrary.BreakRotator` (`SceneComponent.K2_GetComponentRotation` (`self.Cube`))))
  (`parent.ReceiveBeginPlay`)
  (set `self.Return Value X (Roll)` (+ _returnvalue_roll 180.0)))

(event `self.Cube.OnComponentHit`
  (params (HitComponent :type "PrimitiveComponent Object Reference") (OtherActor :type "Actor Object Reference") (OtherComp :type "PrimitiveComponent Object Reference") (NormalImpulse :type "Vector Structure") (Hit :type "HitResult Structure (by ref)")))

(fn `UserConstructionScript`
  (`parent.UserConstructionScript`))