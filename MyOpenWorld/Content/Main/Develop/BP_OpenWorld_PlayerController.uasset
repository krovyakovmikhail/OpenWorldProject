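; Player controller for the open world that toggles a pause menu with the Escape key.
; It creates WBP_PauseMenu on BeginPlay, then pauses or resumes the game, switching mouse cursor and input mode between Game and UI and game only.
; Opening passes the controller to the widget as MainController; closing removes it and hides its settings window and additional buttons panel.
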(event `self.ReceiveBeginPlay`
  (bind _returnvalue (`|CreateWidget` "/Game/Main/UI/Pause_Menu/WBP_PauseMenu.WBP_PauseMenu_C"))
  (set `self.Pause_Widget` _returnvalue))

(event `self.ReceiveEndPlay`
  (params (EndPlayReason :type "EEndPlayReason Enum" :default "Destroyed"))
  (set `self.Pause_Widget` (`self.Pause_Widget`)))

(event `Key|One` :paused true
  (params (Key :type "Key Structure")))

(event `Key|Escape` :paused true
  (params (Key :type "Key Structure"))
  (bind _pause_widget (`self.Pause_Widget`))
  (bind _pause_widget_2 (`self.Pause_Widget`))
  (:`Pressed`
    (if (`self.isPause`)
      (set `self.bShowMouseCursor` false)
      (`GameplayStatics.SetGamePaused` false)
      (set `self.isPause` false)
      (`Widget.RemoveFromParent` (`self.Pause_Widget`))
      (`WidgetBlueprintLibrary.SetInputMode_GameOnly` self)
      (`Widget.SetVisibility` (`/Game/Main/UI/Pause_Menu/WBP_PauseMenu.Target Settings Window` _pause_widget_2) "Hidden")
      (`Widget.SetVisibility` (`/Game/Main/UI/Pause_Menu/WBP_PauseMenu.VerticalBox_additional_buttons` _pause_widget_2) "Hidden")
      (else
        (set `self.bShowMouseCursor` true)
        (`GameplayStatics.SetGamePaused` true)
        (set `self.isPause` true)
        (bind _pause_widget_3 (`self.Pause_Widget`)
          (:`then`
            (`UserWidget.AddToViewport` _pause_widget_3 0)
            (set `/Game/Main/UI/Pause_Menu/WBP_PauseMenu.main_controller` self _pause_widget)
            (`WidgetBlueprintLibrary.SetInputMode_GameAndUIEx` self _pause_widget))
          (:`else`))))))

(fn `UserConstructionScript`)