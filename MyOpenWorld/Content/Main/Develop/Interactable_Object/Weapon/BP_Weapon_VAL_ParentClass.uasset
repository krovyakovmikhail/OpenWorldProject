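; Parent class for pickup guns that an open-world character can carry, aim and fire.
; Interact calls Take, which attaches the gun to the character's Arrow1 and registers it as held; Drop restores physics and detaches it.
; While aiming, Tick line-traces from the muzzle Arrow to position a Sphere marker.
; Fire plays a shot sound and traces likewise, pushing target figures, dartboards or pots, using the impact point as impulse vector.
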(event `InteractableObject_Interface.Interact`
  (params (ActorInteractedWithObject :type "Actor Object Reference"))
  (`self.Take` ActorInteractedWithObject))

(event `self.ReceiveTick`
  (params (DeltaSeconds :type "Float (single-precision)"))
  (bind _sphere (`self.Sphere`))
  (bind _returnvalue (`SceneComponent.K2_GetComponentLocation` (`self.Arrow`)))
  (bind _returnvalue_2 (+ _returnvalue (* (`SceneComponent.GetForwardVector` (`self.Arrow`)) 1500.0)))
  (if (`self.Aiming`)
    (bind _outhit (`KismetSystemLibrary.LineTraceSingle` _returnvalue _returnvalue_2 "TraceTypeQuery1"))
    (if (`GameplayStatics.BreakHitResult` _outhit)
      (`SceneComponent.K2_SetWorldLocation` _sphere (`.Location` (`GameplayStatics.BreakHitResult` _outhit)) false false)
      (else
        (`SceneComponent.K2_SetWorldLocation` _sphere _returnvalue_2 false false)))))

(fn `Drop`
  (returns (Succsess :type Boolean))
  (bind _staticmesh (`self.StaticMesh`))
  (bind _as_bp_open_world_character (`self.As BP Open World Character`))
  (bind _as_bp_open_world_character_2 (`self.As BP Open World Character`)
    (:`then`
      (`PrimitiveComponent.SetSimulatePhysics` _staticmesh true)
      (`PrimitiveComponent.SetCollisionEnabled` _staticmesh "QueryAndPhysics")
      (`self.K2_DetachFromActor` "KeepWorld" "KeepWorld" "KeepWorld")
      (set `/Game/Main/Develop/MAIN_CHAR/blueprint/BP_OpenWorld_Character.Object_In_Hand` null _as_bp_open_world_character)
      (set `/Game/Main/Develop/MAIN_CHAR/blueprint/BP_OpenWorld_Character.Gun in hand` false _as_bp_open_world_character)
      (return false))
    (:`else`)))

(fn `Fire`
  (returns (Succses :type Boolean))
  (bind _returnvalue (`SceneComponent.K2_GetComponentLocation` (`self.Arrow`)))
  (`GameplayStatics.PlaySoundAtLocation` "/Game/Main/Develop/Interactable_Object/Weapon/vintovka-m-14---odin-vyistrel-27852.vintovka-m-14---odin-vyistrel-27852" (`SceneComponent.K2_GetComponentLocation` (`self.Arrow`)) (struct) 1.0 1.0 0.0 null null null)
  (bind _outhit (`KismetSystemLibrary.LineTraceSingle` _returnvalue (+ _returnvalue (* (`SceneComponent.GetForwardVector` (`self.Arrow`)) 1500.0)) "TraceTypeQuery1"))
  (bind _asbp_target_figure (cast `/Game/Main/Develop/Mini_game/SHOOTING_GALLERY/BP_Target_figure` (`.HitActor` (`GameplayStatics.BreakHitResult` _outhit)))
    (:`then`
      (bind _skeletalmesh (`/Game/Main/Develop/Mini_game/SHOOTING_GALLERY/BP_Target_figure.SkeletalMesh` _asbp_target_figure))
      (`PrimitiveComponent.SetSimulatePhysics` _skeletalmesh true)
      (`PrimitiveComponent.AddImpulse` _skeletalmesh (`.ImpactPoint` (`GameplayStatics.BreakHitResult` _outhit)) "None" false)
      (return false))
    (:`CastFailed`
      (bind _asbp_dartboard (cast `/Game/Main/Develop/Mini_game/SHOOTING_GALLERY/BP_dartboard` (`.HitActor` (`GameplayStatics.BreakHitResult` _outhit)))
        (:`then`
          (`PrimitiveComponent.AddImpulse` (`/Game/Main/Develop/Mini_game/SHOOTING_GALLERY/BP_dartboard.Cube` _asbp_dartboard) (`.ImpactPoint` (`GameplayStatics.BreakHitResult` _outhit)) "None" false))
        (:`CastFailed`
          (bind _asbp_pot (cast `/Game/Main/Develop/Mini_game/SHOOTING_GALLERY/BP_Pot` (`.HitActor` (`GameplayStatics.BreakHitResult` _outhit))))
          (`PrimitiveComponent.AddImpulse` (`/Game/Main/Develop/Mini_game/SHOOTING_GALLERY/BP_Pot.Cylinder` _asbp_pot) (`.ImpactPoint` (`GameplayStatics.BreakHitResult` _outhit)) "None" false))))))

(fn `StartAiming`
  (returns (Succsess :type Boolean))
  (set `self.Aiming` true)
  (`SceneComponent.SetVisibility` (`self.Sphere`) true false)
  (return false))

(fn `StopAiming`
  (returns (Succsess :type Boolean))
  (bind _sphere (`self.Sphere`))
  (set `self.Aiming` false)
  (`SceneComponent.SetVisibility` _sphere false false)
  (`SceneComponent.K2_SetWorldLocation` _sphere (`SceneComponent.K2_GetComponentLocation` (`self.Arrow`)) false false)
  (return false))

(fn `Take`
  (params (`Interact Actor` :type "Actor Object Reference"))
  (bind _staticmesh (`self.StaticMesh`))
  (bind _as_bp_open_world_character (`self.As BP Open World Character`))
  (bind _asbp_open_world_character (cast `/Game/Main/Develop/MAIN_CHAR/blueprint/BP_OpenWorld_Character` `Interact Actor`))
  (bind _output_get (set `self.As BP Open World Character` _asbp_open_world_character))
  (`PrimitiveComponent.SetSimulatePhysics` _staticmesh false)
  (`PrimitiveComponent.SetCollisionEnabled` _staticmesh "NoCollision")
  (`self.K2_AttachToComponent` (`/Game/Main/Develop/MAIN_CHAR/blueprint/BP_OpenWorld_Character.Arrow1` _output_get) "None" "SnapToTarget" "SnapToTarget" "SnapToTarget")
  (set `/Game/Main/Develop/MAIN_CHAR/blueprint/BP_OpenWorld_Character.Object_In_Hand` self _as_bp_open_world_character)
  (set `/Game/Main/Develop/MAIN_CHAR/blueprint/BP_OpenWorld_Character.Gun in hand` true _as_bp_open_world_character))

(fn `UserConstructionScript`)