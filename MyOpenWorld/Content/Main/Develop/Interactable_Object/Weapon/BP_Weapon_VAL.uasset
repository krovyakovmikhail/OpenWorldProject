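; BP_Weapon_VAL is an interactable VAL weapon pickup that an open-world character can take in hand and drop.
; Interact calls Take, which casts to BP_OpenWorld_Character, disables mesh physics and collision, and snaps the weapon onto the character's Arrow1 component.
; Take also sets the character's held-object reference and gun flag; Drop clears both, detaches and restores physics and collision.
; The file contains no firing logic.
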(event `InteractableObject_Interface.Interact`
  (params (ActorInteractedWithObject :type "Actor Object Reference"))
  (`self.Take` ActorInteractedWithObject))

(fn `Drop`
  (returns (Succsess :type Boolean))
  (bind _staticmesh (`self.StaticMesh`))
  (bind _as_bp_open_world_character (`self.As BP Open World Character`))
  (bind _as_bp_open_world_character_2 (`self.As BP Open World Character`)
    (:`then`
      (`PrimitiveComponent.SetSimulatePhysics` _staticmesh true)
      (`PrimitiveComponent.SetCollisionEnabled` _staticmesh "QueryAndPhysics")
      (`self.K2_DetachFromActor` "KeepWorld" "KeepWorld" "KeepWorld")
      (set `/Game/Main/Develop/MAIN_CHAR/blueprint/BP_OpenWorld_Character.Object_In_Hand` null _as_bp_open_world_character)
      (set `/Game/Main/Develop/MAIN_CHAR/blueprint/BP_OpenWorld_Character.Gun in hand` false _as_bp_open_world_character)
      (return false))
    (:`else`)))

(fn `Take`
  (params (`Interact Actor` :type "Actor Object Reference"))
  (bind _staticmesh (`self.StaticMesh`))
  (bind _as_bp_open_world_character (`self.As BP Open World Character`))
  (bind _asbp_open_world_character (cast `/Game/Main/Develop/MAIN_CHAR/blueprint/BP_OpenWorld_Character` `Interact Actor`))
  (bind _output_get (set `self.As BP Open World Character` _asbp_open_world_character))
  (`PrimitiveComponent.SetSimulatePhysics` _staticmesh false)
  (`PrimitiveComponent.SetCollisionEnabled` _staticmesh "NoCollision")
  (`self.K2_AttachToComponent` (`/Game/Main/Develop/MAIN_CHAR/blueprint/BP_OpenWorld_Character.Arrow1` _output_get) "None" "SnapToTarget" "SnapToTarget" "SnapToTarget")
  (set `/Game/Main/Develop/MAIN_CHAR/blueprint/BP_OpenWorld_Character.Object_In_Hand` self _as_bp_open_world_character)
  (set `/Game/Main/Develop/MAIN_CHAR/blueprint/BP_OpenWorld_Character.Gun in hand` true _as_bp_open_world_character))

(fn `UserConstructionScript`)