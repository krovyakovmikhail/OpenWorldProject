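; Interactable scuba gear that an open-world character can put on.
; On Interact it casts the actor to BP_OpenWorld_Character and branches on its ThereIsScubaGear flag, which this Blueprint never sets.
; Putting on disables the Balloon component's physics and collision, then calls a snap attach to SpineSocket, using the character's root component as parent.
; The take-off function is an empty stub.
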(event `InteractableObject_Interface.Interact`
  (params (ActorInteractedWithObject :type "Actor Object Reference"))
  (bind _asbp_open_world_character (cast `/Game/Main/Develop/MAIN_CHAR/blueprint/BP_OpenWorld_Character` ActorInteractedWithObject))
  (if (`/Game/Main/Develop/MAIN_CHAR/blueprint/BP_OpenWorld_Character.There is scuba gear` _asbp_open_world_character)
    (`self.take off` ActorInteractedWithObject)
    (else
      (`self.Put On` ActorInteractedWithObject))))

(fn `Put On`
  (params (Actor :type "Actor Object Reference"))
  (bind _balloon (`self.Balloon`))
  (`PrimitiveComponent.SetSimulatePhysics` _balloon false)
  (`PrimitiveComponent.SetCollisionEnabled` _balloon "NoCollision")
  (`self.K2_AttachToComponent` (`Actor.RootComponent` Actor) "SpineSocket" "SnapToTarget" "SnapToTarget" "SnapToTarget"))

(fn `take off`
  (params (Actor :type "Actor Object Reference")))

(fn `UserConstructionScript`)