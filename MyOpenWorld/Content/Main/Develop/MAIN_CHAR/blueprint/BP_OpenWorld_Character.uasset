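; Open-world player character that walks, sprints, picks up items, fires weapons and ragdolls when health runs out.
; Capsule overlaps query objects through interface messages instead of casts, separating interactables, liftable items and vehicles, and update the UI widget's prompt.
; Interaction attaches liftables to the hand, or guns to an arrow component.
; Right mouse aims with a camera zoom, and its release throws throwable non-gun items by impulse, while Q drops them.
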(event `self.ReceiveBeginPlay`
  ;[0.3 0.55 0.9 0.4] Begin  play
  (bind _returnvalue (`|CreateWidget` "/Game/Main/UI/Main_Character_Interface/WBP_Main_User_Interface.WBP_Main_User_Interface_C"))
  (bind _output_get (set `self.User_interface_widget` _returnvalue))
  (`UserWidget.AddToPlayerScreen` _output_get 0))

(event `self.ReceiveTick`
  (params (DeltaSeconds :type "Float (single-precision)"))
  (bind _returnvalue (`self.GetVelocity`))
  ;[1 0 0] Tick\
  (if (<= (`self.Health`) 0.0)
    (`PrimitiveComponent.SetSimulatePhysics` (`self.Mesh`) true)
    (`CharacterMovementComponent.DisableMovement` (`self.CharacterMovement`))
    (else
      (`|ExecutionSequence`
        (:`then_0`
          (bind _weapon (`self.Weapon`)
            (:`then`
              (set `self.shoot` (`/Game/Main/Develop/MAIN_CHAR/blueprint/BP_OpenWorld_Character.Shoot` _weapon)))
            (:`else`)))
        (:`then_1`
          (if (> (`KismetMathLibrary.VSize` _returnvalue) 0.0)
            (set `self.onWalk` true)
            (set `self.Forward speed` (`KismetMathLibrary.Dot_VectorVector` _returnvalue (`self.GetActorForwardVector`)))
            (else
              (set `self.onWalk` false))))))))

(event `self.CapsuleComponent.OnComponentBeginOverlap`
  (params (OverlappedComponent :type "PrimitiveComponent Object Reference") (OtherActor :type "Actor Object Reference") (OtherComp :type "PrimitiveComponent Object Reference") (OtherBodyIndex :type Integer) (bFromSweep :type Boolean) (SweepResult :type "HitResult Structure (by ref)"))
  ;[0.5662 1 0.3728] Вместо Cast to использую общение через интерфес Interaction_Object_Interfase. Пока предполагается 3 класса использующие этот интерфейс: BP_Interaction_object - предмет с которым можно взаимодействовать, BP_Lifted_item - который можно поднять. wheeled vehicle - транспортное средство. (Здесь предполагается типа колесные ТС, нужно расширить или замениьэтот клас )
  ;;[1 1 1] Overlap
  (if (`KismetSystemLibrary.DoesImplementInterface` OtherActor)
    (if (!= OtherActor (`self.Object_In_Hand`))
      ;;;[1 0.1823 0.1823] Задаем вопрос ты что за предмет?
      (bind _object (message `/Game/Main/Develop/MAIN_CHAR/blueprint/BP_OpenWorld_Character.WhoAreYou` OtherActor))
      ;;;[1 1 1] Если ответ был, получим ссылку на клас BP_Interaction_object - это либо поднимаемые предметы, либо с которыми можно повзаимодействовать
      (bind _output_get (set `self.Interaction_object` _object))
      (bind _interaction_object (`self.Interaction_object`)
        (:`then`
          ;;;[1 1 1] Если его можно взять в руку то это предмет класса BP_Lifted_item, если да то уточняющий вопрос что бы получить ссылку на класс.
          (if (`/Game/Main/Develop/MAIN_CHAR/blueprint/BP_OpenWorld_Character.You can take` _interaction_object)
            (`self.Lifted_Object`
              (:`then`)
              (:`else`
                (bind _lifted_object (`self.Concretize yourself` _output_get))
                (bind _output_get_2 (set `self.Lifted_Object` _lifted_object))
                (`/Game/Main/UI/Main_Character_Interface/WBP_Main_User_Interface.Set Interact Text` (`self.User_interface_widget`) null _output_get_2 null null)))))
        (:`else`
          ;;;[1 1 1] Если ответ на ворос не прошел, значит это ТС. т.к  транспортные средства будут класса wheeled vehicle
          (message `/Game/Main/Develop/MAIN_CHAR/blueprint/BP_OpenWorld_Character.What A Car` OtherActor))))))

(event `Key|LeftShift`
  (params (Key :type "Key Structure"))
  ;[1 1 1] Motion control
  (:`Pressed`
    (set `self.Updatespeed` true))
  (:`Released`
    (set `self.Updatespeed` false)))

(event `InputAxis|MoveForward`
  (params (AxisValue :type "Float (single-precision)"))
  ;[1 1 1] Motion control
  (`self.AddMovementInput` (`self.GetActorForwardVector`) AxisValue)
  (if (< (`self.Forward speed`) 0.0)
    (set `CharacterMovementComponent.MaxWalkSpeed` 300.0 (`self.CharacterMovement`))
    (elif (`self.Updatespeed`)
      (set `CharacterMovementComponent.MaxWalkSpeed` 600.0 (`self.CharacterMovement`))
      (else
        (set `CharacterMovementComponent.MaxWalkSpeed` 450.0 (`self.CharacterMovement`))))))

(event `self.CapsuleComponent.OnComponentEndOverlap`
  (params (OverlappedComponent :type "PrimitiveComponent Object Reference") (OtherActor :type "Actor Object Reference") (OtherComp :type "PrimitiveComponent Object Reference") (OtherBodyIndex :type Integer))
  ;[0.5662 1 0.3728] Вместо Cast to использую общение через интерфес Interaction_Object_Interfase. Пока предполагается 3 класса использующие этот интерфейс: BP_Interaction_object - предмет с которым можно взаимодействовать, BP_Lifted_item - который можно поднять. wheeled vehicle - транспортное средство. (Здесь предполагается типа колесные ТС, нужно расширить или замениьэтот клас )
  ;;[1 1 1] Overlap
  (if (`KismetSystemLibrary.DoesImplementInterface` OtherActor)
    (if (!= OtherActor (`self.Object_In_Hand`))
      (set `self.Interaction_object` null)
      (bind _output_get (set `self.Lifted_Object` null))
      (`/Game/Main/UI/Main_Character_Interface/WBP_Main_User_Interface.Set Interact Text` (`self.User_interface_widget`) null _output_get null null))))

(event `InputAction|Interaction`
  (params (Key :type "Key Structure"))
  ;[0.09448 0 1] Interaction and dropi item
  (:`Pressed`
    (bind _interaction_object (`self.Interaction_object`)
      (:`then`
        (message `/Game/Main/Develop/MAIN_CHAR/blueprint/BP_OpenWorld_Character.Interaction` _interaction_object)
        (bind _lifted_object (`self.Lifted_Object`)
          (:`then`
            (`self.Take Interact Item` _lifted_object))
          (:`else`)))
      (:`else`))))

(event `Key|LeftMouseButton`
  (params (Key :type "Key Structure"))
  ;[1 1 1] Обработка ввода кнопок мыши
  (:`Pressed`
    (if (not (`self.shoot`))
      (`self.Object_In_Hand`
        (:`then`
          (bind _weapon (`self.Weapon`)
            (:`then`
              (`self.Fire` _weapon))
            (:`else`)))
        (:`else`)))))

(event `Key|Q`
  (params (Key :type "Key Structure"))
  ;[0.09448 0 1] Interaction and dropi item
  (:`Pressed`
    (`self.DropItemInHand`)))

(event `Key|RightMouseButton`
  (params (Key :type "Key Structure"))
  (bind _springarmcomponent (`self.SpringArmComponent`))
  ;[1 1 1] Обработка ввода кнопок мыши
  (:`Pressed`
    (`self.Object_In_Hand`
      (:`then`
        (set `self.onAIM` true)
        (set `self.bUseControllerRotationPitch` true)
        (`self.AIM` (`self.Object_In_Hand`) self)
        (set `SpringArmComponent.TargetArmLength` (`KismetMathLibrary.Lerp` (`SpringArmComponent.TargetArmLength` _springarmcomponent) 100.0 1.1) _springarmcomponent))
      (:`else`)))
  (:`Released`
    (set `self.bUseControllerRotationPitch` false)
    (bind _object_in_hand (`self.Object_In_Hand`)
      (:`then`
        (set `SpringArmComponent.TargetArmLength` (`KismetMathLibrary.Lerp` (`SpringArmComponent.TargetArmLength` (`self.SpringArmComponent`)) 250.0 1.5) (`self.SpringArmComponent`))
        (set `self.onAIM` false)
        (if (`/Game/Main/Develop/MAIN_CHAR/blueprint/BP_OpenWorld_Character.Can throw` _object_in_hand)
          (if (`self.Gun in hand`)
            (bind _weapon (`self.Weapon`)
              (:`then`
                (`self.End of aiming` _weapon))
              (:`else`))
            (else
              (set `self.throw` true)
              (`KismetSystemLibrary.Delay` 0.2)
              (`self.Throw An Item` (`self.Object_In_Hand`))
              (`KismetSystemLibrary.Delay` 0.5)
              (set `self.throw` false)))))
      (:`else`))))

(event `Key|Z`
  (params (Key :type "Key Structure"))
  (:`Pressed`
    (`PrimitiveComponent.SetCollisionEnabled` (`self.CapsuleComponent`) "NoCollision")
    (`PrimitiveComponent.SetSimulatePhysics` (`self.Mesh`) true)))

(fn `DropItemInHand`
  (bind _object_in_hand (`self.Object_In_Hand`)
    (:`then`
      (bind _rooot (`/Game/Main/Develop/MAIN_CHAR/blueprint/BP_OpenWorld_Character.Rooot` _object_in_hand))
      (`PrimitiveComponent.SetCollisionEnabled` _rooot "PhysicsOnly")
      (`PrimitiveComponent.SetSimulatePhysics` _rooot true)
      (`self.K2_DetachFromActor` _object_in_hand "KeepWorld" "KeepWorld" "KeepWorld")
      (set `ProjectileMovementComponent.ProjectileGravityScale` 1.0 (`/Game/Main/Develop/MAIN_CHAR/blueprint/BP_OpenWorld_Character.ProjectileMovement` _object_in_hand))
      (set `self.Gun in hand` false)
      (set `self.Object_In_Hand` null)
      (`self.Interaction_object`
        (:`then`
          (set `self.Interaction_object` null)
          (set `self.Weapon` null)
          (`/Game/Main/UI/Main_Character_Interface/WBP_Main_User_Interface.Set Interact Text` (`self.User_interface_widget`) null null null (`self.Object_In_Hand`)))
        (:`else`)))
    (:`else`)))

(fn `Take Interact Item`
  (params (`the object being lifted` :type "Object Object Reference"))
  (returns (Succsess :type Boolean))
  (bind _rooot (`/Game/Main/Develop/MAIN_CHAR/blueprint/BP_OpenWorld_Character.Rooot` `the object being lifted`))
  (`self.Object_In_Hand`
    (:`then`)
    (:`else`
      (if (`/Game/Main/Develop/MAIN_CHAR/blueprint/BP_OpenWorld_Character.is it a weapon?` `the object being lifted`)
        (set `self.Gun in hand` true)
        (bind _weapon (message `/Game/Main/Develop/MAIN_CHAR/blueprint/BP_OpenWorld_Character.What A Weapon` `the object being lifted`))
        (set `self.Object_In_Hand` _weapon)
        (set `self.Weapon` _weapon))
      (set `ProjectileMovementComponent.ProjectileGravityScale` 0.0 (`/Game/Main/Develop/MAIN_CHAR/blueprint/BP_OpenWorld_Character.ProjectileMovement` `the object being lifted`))
      (`PrimitiveComponent.SetSimulatePhysics` _rooot false)
      (`PrimitiveComponent.SetCollisionEnabled` _rooot "NoCollision")
      (if (`self.Gun in hand`)
        (`self.K2_AttachToComponent` `the object being lifted` (`self.Arrow1`) "None" "SnapToTarget" "SnapToTarget" "SnapToTarget" true)
        (else
          (`self.K2_AttachToComponent` `the object being lifted` (`self.Hand_R`) "None" "SnapToTarget" "SnapToTarget" "SnapToTarget" true)))
      (bind _output_get (set `self.Object_In_Hand` (`self.Lifted_Object`)))
      (`/Game/Main/UI/Main_Character_Interface/WBP_Main_User_Interface.Set Interact Text` (`self.User_interface_widget`) null null null _output_get)
      (set `self.Lifted_Object` null)
      (return true))))

(fn `Throw An Item`
  (params (`Onject in hand` :type "Object Object Reference"))
  (returns (Succsses :type Boolean))
  (bind _returnvalue (`self.GetActorForwardVector`))
  (bind _object_in_hand (`self.Object_In_Hand`)
    (:`then`
      (bind _rooot (`/Game/Main/Develop/MAIN_CHAR/blueprint/BP_OpenWorld_Character.Rooot` _object_in_hand))
      (`PrimitiveComponent.SetCollisionEnabled` _rooot "PhysicsOnly")
      (`PrimitiveComponent.SetSimulatePhysics` _rooot true)
      (`self.K2_DetachFromActor` _object_in_hand "KeepWorld" "KeepWorld" "KeepWorld")
      (set `ProjectileMovementComponent.ProjectileGravityScale` 1.0 (`/Game/Main/Develop/MAIN_CHAR/blueprint/BP_OpenWorld_Character.ProjectileMovement` _object_in_hand))
      (`self.K2_AddActorLocalOffset` _object_in_hand (/ _returnvalue 2.0) false false)
      (`PrimitiveComponent.AddImpulse` _rooot (+ (* _returnvalue 2000.0) (* (`self.GetActorUpVector`) 300.0)) "None" false)
      (`self.throw` _object_in_hand)
      (`self.Event Explosion ` _object_in_hand)
      (set `self.Object_In_Hand` null)
      (`self.Interaction_object`
        (:`then`
          (set `self.Interaction_object` null)
          (set `self.Weapon` null)
          (`/Game/Main/UI/Main_Character_Interface/WBP_Main_User_Interface.Set Interact Text` (`self.User_interface_widget`) null null null (`self.Object_In_Hand`))
          (return true))
        (:`else`)))
    (:`else`)))

(fn `UserConstructionScript`)