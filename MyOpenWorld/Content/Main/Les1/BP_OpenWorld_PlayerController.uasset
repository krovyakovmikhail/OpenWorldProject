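; Player controller for the open world level that toggles a pause menu when the 1 key is pressed.
; Pausing shows the cursor, creates WBP_PauseMenu, passes it a reference to this controller and switches to Game and UI input focused on the menu.
; Unpausing hides the cursor, removes and clears the widget and restores game-only input, with an IsPause flag tracking the state.
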(event `self.ReceiveBeginPlay`)

(event `Key|Escape` :paused true
  (params (Key :type "Key Structure")))

(event `Key|One` :paused true
  (params (Key :type "Key Structure"))
  (bind _pause_widget (`self.Pause_Widget`))
  (:`Pressed`
    (if (`self.isPause`)
      (set `self.bShowMouseCursor` false)
      (`GameplayStatics.SetGamePaused` false)
      (set `self.isPause` false)
      (`Widget.RemoveFromParent` (`self.Pause_Widget`))
      (set `self.Pause_Widget` null)
      (`WidgetBlueprintLibrary.SetInputMode_GameOnly` self)
      (else
        (set `self.bShowMouseCursor` true)
        (`GameplayStatics.SetGamePaused` true)
        (set `self.isPause` true)
        (bind _returnvalue (`|CreateWidget` "/Game/Main/les2/Pause_Menu/WBP_PauseMenu.WBP_PauseMenu_C"))
        (bind _output_get (set `self.Pause_Widget` _returnvalue))
        (`UserWidget.AddToViewport` _output_get 0)
        (set `/Game/Main/les2/Pause_Menu/WBP_PauseMenu.main_controller` self _pause_widget)
        (`WidgetBlueprintLibrary.SetInputMode_GameAndUIEx` self _pause_widget)))))

(fn `UserConstructionScript`)